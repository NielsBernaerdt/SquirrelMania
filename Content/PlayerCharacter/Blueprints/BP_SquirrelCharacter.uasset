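; BP_SquirrelCharacter is the squirrel player character Blueprint, handling one-way platform collision and a jetpack sound.
; Each tick it sets two custom capsule channels to Block only when not rising, stunned, falling through or stuck; otherwise to Ignore.
; StuckCollision overlaps with PlatformBase actors drive the stuck flag.
; Ending overlap with a BP_Jetpack spawns a jetpack sound at world origin and destroys it three seconds later.
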(event `self.ReceiveActorEndOverlap`
  (params (OtherActor :type "Actor Object Reference"))
  (if (== (`GameplayStatics.GetObjectClass` OtherActor) "/Game/GamePlayObjects/Blueprints/BP_Jetpack.BP_Jetpack_C")
    (bind _returnvalue (`GameplayStatics.SpawnSoundAtLocation` "/Game/Sound/Jetpack/SE_Jetpack.SE_Jetpack" (0.0 0.0 0.0) (struct) 0.25 1.0 0.0 null null))
    (`KismetSystemLibrary.Delay` 3.0)
    (`ActorComponent.K2_DestroyComponent` _returnvalue)))

(event `self.ReceiveActorBeginOverlap`
  (params (OtherActor :type "Actor Object Reference")))

(event `self.ReceiveBeginPlay`)

(event `self.ReceiveTick`
  (params (DeltaSeconds :type "Float (single-precision)"))
  (bind (_returnvalue_x _returnvalue_y _returnvalue_z) (`KismetMathLibrary.BreakVector` (`self.GetVelocity`)))
  (if (`self.isInStuckRange`)
    (`PrimitiveComponent.SetCollisionResponseToChannel` (`self.CapsuleComponent`) "ECC_GameTraceChannel1" "ECR_Ignore")
    (`PrimitiveComponent.SetCollisionResponseToChannel` (`self.CapsuleComponent`) "ECC_GameTraceChannel2" "ECR_Ignore")
    (else
      ;[1 1 1] StunCheck
      (if (`self.m_bStunned`)
        (`PrimitiveComponent.SetCollisionResponseToChannel` (`self.CapsuleComponent`) "ECC_GameTraceChannel1" "ECR_Ignore")
        (`PrimitiveComponent.SetCollisionResponseToChannel` (`self.CapsuleComponent`) "ECC_GameTraceChannel2" "ECR_Ignore")
        (else
          ;[1 1 1] FallingThrough Check
          (if (`self.m_FallingThrough`)
            (`PrimitiveComponent.SetCollisionResponseToChannel` (`self.CapsuleComponent`) "ECC_GameTraceChannel1" "ECR_Ignore")
            (`PrimitiveComponent.SetCollisionResponseToChannel` (`self.CapsuleComponent`) "ECC_GameTraceChannel2" "ECR_Ignore")
            (else
              ;[1 1 1] Velocity Check
              (if (<= _returnvalue_z 0.0)
                (`PrimitiveComponent.SetCollisionResponseToChannel` (`self.CapsuleComponent`) "ECC_GameTraceChannel1" "ECR_Block")
                (`PrimitiveComponent.SetCollisionResponseToChannel` (`self.CapsuleComponent`) "ECC_GameTraceChannel2" "ECR_Block")
                (else
                  (`PrimitiveComponent.SetCollisionResponseToChannel` (`self.CapsuleComponent`) "ECC_GameTraceChannel1" "ECR_Ignore")
                  (`PrimitiveComponent.SetCollisionResponseToChannel` (`self.CapsuleComponent`) "ECC_GameTraceChannel2" "ECR_Ignore"))))))))))

(event `self.StuckCollision.OnComponentBeginOverlap`
  (params (OverlappedComponent :type "PrimitiveComponent Object Reference") (OtherActor :type "Actor Object Reference") (OtherComp :type "PrimitiveComponent Object Reference") (OtherBodyIndex :type Integer) (bFromSweep :type Boolean) (SweepResult :type "HitResult Structure (by ref)"))
  (cast `PlatformBase` OtherActor)
  (set `self.isInStuckRange` true))

(event `self.StuckCollision.OnComponentEndOverlap`
  (params (OverlappedComponent :type "PrimitiveComponent Object Reference") (OtherActor :type "Actor Object Reference") (OtherComp :type "PrimitiveComponent Object Reference") (OtherBodyIndex :type Integer))
  (cast `PlatformBase` OtherActor)
  (set `self.isInStuckRange` false))

(fn `UserConstructionScript`)