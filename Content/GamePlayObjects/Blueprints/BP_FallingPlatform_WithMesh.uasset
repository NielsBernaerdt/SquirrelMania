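; Falling platform actor that drops after a character steps on it and knocks back characters it hits.
; Feet collision overlapping the box triggers, after a short delay, mesh physics simulation and overlap-only collision.
; A second delay enables the initially ignored DamageBox, so the faster-falling character is not hit immediately.
; While falling, DamageBox launches non-dodging characters along world Y, away from the platform's position.
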(event `self.ReceiveBeginPlay`
  (`PrimitiveComponent.SetCollisionResponseToAllChannels` (`self.DamageBox`) "ECR_Ignore"))

(event `self.Box.OnComponentBeginOverlap`
  (params (OverlappedComponent :type "PrimitiveComponent Object Reference") (OtherActor :type "Actor Object Reference") (OtherComp :type "PrimitiveComponent Object Reference") (OtherBodyIndex :type Integer) (bFromSweep :type Boolean) (SweepResult :type "HitResult Structure (by ref)"))
  (bind _staticmesh (`self.StaticMesh`))
  (bind _asbp_char_squirrel (cast `` OtherActor))
  (if (== OtherComp (`/Game/GamePlayObjects/Blueprints/BP_FallingPlatform_WithMesh.FeetCollision` _asbp_char_squirrel))
    (`KismetSystemLibrary.Delay` 0.5)
    (`KismetSystemLibrary.PrintString` "Falling")
    (set `self.isFalling` true)
    (`PrimitiveComponent.SetSimulatePhysics` _staticmesh true)
    (`PrimitiveComponent.SetCollisionResponseToAllChannels` _staticmesh "ECR_Overlap")
    (`KismetSystemLibrary.Delay` 0.5)
    ;[1 1 1] Only start checking here so the actor doesnt get hit immediately when the platform starts falling (actor falls faster)
    (`PrimitiveComponent.SetCollisionResponseToAllChannels` (`self.DamageBox`) "ECR_Overlap")))

(event `self.DamageBox.OnComponentBeginOverlap`
  (params (OverlappedComponent :type "PrimitiveComponent Object Reference") (OtherActor :type "Actor Object Reference") (OtherComp :type "PrimitiveComponent Object Reference") (OtherBodyIndex :type Integer) (bFromSweep :type Boolean) (SweepResult :type "HitResult Structure (by ref)"))
  (bind (_returnvalue_x _returnvalue_y) (`KismetMathLibrary.BreakVector` (`self.K2_GetActorLocation`)))
  (bind _asbp_char_squirrel (cast `` OtherActor))
  (if (`/Game/GamePlayObjects/Blueprints/BP_FallingPlatform_WithMesh.isDodging` _asbp_char_squirrel)
    _
    (elif (`self.isFalling`)
      (`KismetSystemLibrary.PrintString` "Obstacle hit")
      (bind (_returnvalue_x_2 _returnvalue_y_2) (`KismetMathLibrary.BreakVector` (`self.K2_GetActorLocation` _asbp_char_squirrel)))
      (if (> _returnvalue_y_2 _returnvalue_y)
        (`Character.LaunchCharacter` _asbp_char_squirrel (0.0 2000.0 0.0) true false)
        (else
          (`Character.LaunchCharacter` _asbp_char_squirrel (0.0 -2000.0 0.0) true false))))))

(fn `UserConstructionScript`)